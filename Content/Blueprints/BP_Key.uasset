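; BP_Key is a collectible key part that spins continuously until the player character overlaps its collision.
; On pickup it increments KeyParts on BP_FirstPersonCharacter, sets HasKey once that count equals the number of keys in the level, then destroys itself.
; Each key caches all BP_Key actors at BeginPlay, so the required total scales with how many are present in the level.
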(event OnComponentBeginOverlap(Collision)
  (params (OverlappedComponent :type Primitive%20Component%20Object%20Reference) (OtherActor :type Actor%20Object%20Reference) (OtherComp :type Primitive%20Component%20Object%20Reference) (OtherBodyIndex :type Integer) (bFromSweep :type Boolean) (SweepResult :type Hit%20Result%20Structure%20%28by%20ref%29))
  (if (== OtherActor (Game|GetPlayerCharacter 0))
    ;[0.15 0.15 0.15 0.5] si se quiere hacer +1 accion a la vez
    (Utilities|FlowControl|Sequence
      (:then_0
        ;[0.15 0.15 0.15 0.5] +1 llave
        (bind _output_get (Variables|/Game/FirstPerson/Blueprints/BP_FirstPersonCharacter.BP_FirstPersonCharacter_C|SetKeyParts (.AsBP%20First%20Person%20Character (Utilities|Casting|CastToBP_FirstPersonCharacter (Game|GetPlayerCharacter 0))) (Variables|/Game/FirstPerson/Blueprints/BP_FirstPersonCharacter.BP_FirstPersonCharacter_C|GetKeyParts (.AsBP%20First%20Person%20Character (Utilities|Casting|CastToBP_FirstPersonCharacter (Game|GetPlayerCharacter 0))))))
        (Math|Integer|IncrementInt _output_get))
      (:then_1
        ;[0.15 0.15 0.15 0.5] si la cantidad de llaves coleccionadas == las llaves del nivel entonces hasKey = true
        (if (== (Variables|/Game/FirstPerson/Blueprints/BP_FirstPersonCharacter.BP_FirstPersonCharacter_C|GetKeyParts (.AsBP%20First%20Person%20Character (Utilities|Casting|CastToBP_FirstPersonCharacter (Game|GetPlayerCharacter 0)))) (Utilities|Array|Length (stale EventBeginPlay _outactors)))
          (Variables|/Game/FirstPerson/Blueprints/BP_FirstPersonCharacter.BP_FirstPersonCharacter_C|SetHasKey (.AsBP%20First%20Person%20Character (Utilities|Casting|CastToBP_FirstPersonCharacter (Game|GetPlayerCharacter 0))) true)))
      (:then_2
        ;[0.15 0.15 0.15 0.5] destruye
        (Actor|DestroyActor)))))

(event EventBeginPlay
  ;[0.15 0.15 0.15 0.5] si la cantidad de llaves coleccionadas == las llaves del nivel entonces hasKey = true
  ;;[0.15 0.15 0.15 0.5] hace que sea escalable porque pilla todas las llaves del nivel
  ;;;[0.1478 0 0.15 0.5] start
  (bind _outactors (Actor|GetAllActorsOfClass "BP_Key_C")))

(event Collision|EventActorBeginOverlap
  (params (OtherActor :type Actor%20Object%20Reference)))

(event EventTick
  (params (DeltaSeconds :type Float%20%28single-precision%29))
  ;[0.149 0 0.15 0.5] update
  ;;[0.15 0.15 0.15 0.5] rota
  (Transformation|AddLocalRotation (Variables|Default|Getkey) (Math|Rotator|MakeRotator 0.0 (* DeltaSeconds 9e+01) 0.0) false false))

(fn ConstructionScript)