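; Target dummy for a shooting-range minigame, keeping TargetsLeft and the win flag on BP_FirstPersonCharacter.
; A hit during practice tips it over by timeline, decrements the count and either wins at zero or raises it again after a delay.
; InitializeShootingRange registers and raises it, randomly starting a lerped slide along X; StayDown lays it flat and stops movement.
; A DoOnce, reset through Recover, guards against repeat hits.
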(event Custom|DummyMovement
  (if (Variables|Default|GetshouldMove)
    (bind _movedummy (Timeline|Movement Play)
      (:Update
        (Transformation|SetActorLocation (Math|Vector|Lerp(Vector) (Variables|Default|GetInitialPos) (Variables|Default|GetFinalPos) _movedummy) false false)))
    (else
      (Timeline|Movement Stop))))

(event Custom|InitializeShootingRange
  (bind _bp_firstperson (Variables|Default|GetBP_FirstPerson))
  (bind _output_get (Variables|/Game/FirstPerson/Blueprints/BP_FirstPersonCharacter.BP_FirstPersonCharacter_C|SetTargetsLeft _bp_firstperson (Variables|/Game/FirstPerson/Blueprints/BP_FirstPersonCharacter.BP_FirstPersonCharacter_C|GetTargetsLeft _bp_firstperson)))
  (Math|Integer|IncrementInt _output_get
    (:%20%20
      (Variables|Default|SetisDown false)
      (CallFunction|Recover)
      (if (== (.roll (Transformation|GetActorRotation)) -85.0)
        (bind _rotatedummy (Timeline|Initialize ReverseFromEnd)
          (:Update
            (Transformation|SetActorRotation (Math|Rotator|MakeRotator _rotatedummy 0.0 0.0)))
          (:Finished
            (if (>= (Math|Random|RandomIntegerinRange 0 10) 6) :!label _label
              (Variables|Default|SetshouldMove true)
              (CallFunction|DummyMovement))))
        (else
          (goto _label))))))

(event Custom|HitBehaviour
  (bind _bp_firstperson (Variables|Default|GetBP_FirstPerson))
  (bind _bp_firstperson_2 (Variables|Default|GetBP_FirstPerson))
  (bind _bp_firstperson_3 (Variables|Default|GetBP_FirstPerson))
  (bind _bp_firstperson_4 (Variables|Default|GetBP_FirstPerson))
  (if (Math|Boolean|ANDBoolean (== (Variables|/Game/FirstPerson/Blueprints/BP_FirstPersonCharacter.BP_FirstPersonCharacter_C|GetShootingPracticeWon _bp_firstperson_4) false) (not (Variables|Default|GetisDown)) (== (Variables|/Game/FirstPerson/Blueprints/BP_FirstPersonCharacter.BP_FirstPersonCharacter_C|GetShootingPracticeBegun _bp_firstperson_4) true))
    (Utilities|FlowControl|DoOnce false
      (:Completed
        (Variables|Default|SetisDown true)
        (bind _rotatedummy (Timeline|Hit PlayFromStart)
          (:Update
            (Transformation|SetActorRotation (Math|Rotator|MakeRotator _rotatedummy 0.0 0.0)))
          (:Finished
            (bind _output_get (Variables|/Game/FirstPerson/Blueprints/BP_FirstPersonCharacter.BP_FirstPersonCharacter_C|SetTargetsLeft _bp_firstperson_3 (Variables|/Game/FirstPerson/Blueprints/BP_FirstPersonCharacter.BP_FirstPersonCharacter_C|GetTargetsLeft _bp_firstperson_3)))
            (Math|Integer|DecrementInt _output_get
              (:%20%20
                (if (== (Variables|/Game/FirstPerson/Blueprints/BP_FirstPersonCharacter.BP_FirstPersonCharacter_C|GetTargetsLeft (Variables|Default|GetBP_FirstPerson)) 0)
                  (Variables|/Game/FirstPerson/Blueprints/BP_FirstPersonCharacter.BP_FirstPersonCharacter_C|SetShootingPracticeWon (Variables|Default|GetBP_FirstPerson) true)
                  (elif (and (== (Variables|/Game/FirstPerson/Blueprints/BP_FirstPersonCharacter.BP_FirstPersonCharacter_C|GetShootingPracticeWon _bp_firstperson) true) (== (Variables|/Game/FirstPerson/Blueprints/BP_FirstPersonCharacter.BP_FirstPersonCharacter_C|GetShootingPracticeBegun _bp_firstperson) true))
                    (CallFunction|Recover)
                    (else
                      (Utilities|FlowControl|Delay 1e+01)
                      (bind _rotatedummy_2 (Timeline|RecoverHit ReverseFromEnd)
                        (:Update
                          (Transformation|SetActorRotation (Math|Rotator|MakeRotator _rotatedummy_2 0.0 0.0)))
                        (:Finished
                          (if (and (== (Variables|/Game/FirstPerson/Blueprints/BP_FirstPersonCharacter.BP_FirstPersonCharacter_C|GetShootingPracticeBegun _bp_firstperson_2) true) (not (Variables|/Game/FirstPerson/Blueprints/BP_FirstPersonCharacter.BP_FirstPersonCharacter_C|GetShootingPracticeWon _bp_firstperson_2)))
                            (bind _output_get_2 (Variables|/Game/FirstPerson/Blueprints/BP_FirstPersonCharacter.BP_FirstPersonCharacter_C|SetTargetsLeft _bp_firstperson_2 (Variables|/Game/FirstPerson/Blueprints/BP_FirstPersonCharacter.BP_FirstPersonCharacter_C|GetTargetsLeft _bp_firstperson_2)))
                            (Math|Integer|IncrementInt _output_get_2
                              (:%20%20
                                (Variables|Default|SetisDown false)
                                (CallFunction|Recover)))
                            (else
                              (CallFunction|Recover))))))))))))))))

(event Custom|Recover
  (bind _bp_firstperson (Variables|Default|GetBP_FirstPerson))
  (bind _bp_firstperson_2 (Variables|Default|GetBP_FirstPerson))
  (bind _bp_firstperson_3 (Variables|Default|GetBP_FirstPerson))
  (Utilities|FlowControl|DoOnce false) ; enters at Reset
)

(event Custom|StayDown
  (if (not (== (.roll (Transformation|GetActorRotation)) -85.0))
    (bind _rotatedummy (Timeline|StayDowned PlayFromStart)
      (:Update
        (Transformation|SetActorRotation (Math|Rotator|MakeRotator _rotatedummy 0.0 0.0)))
      (:Finished
        (Variables|Default|SetshouldMove false)
        (CallFunction|DummyMovement)))))

(event EventBeginPlay
  (bind _returnvalue (Math|Random|RandomFloatinRange 3e+02 6e+02))
  (bind _returnvalue_2 (Transformation|GetActorLocation))
  (Utilities|FlowControl|Sequence
    (:then_0
      (if (> (.x (Transformation|GetActorLocation)) 1.6e+02)
        (bind _output_get (Variables|Default|SetInitialPos _returnvalue_2))
        (Variables|Default|SetFinalPos (- _output_get (Math|Vector|MakeVector _returnvalue 0.0 0.0)))
        (else
          (bind _output_get_2 (Variables|Default|SetInitialPos _returnvalue_2))
          (Variables|Default|SetFinalPos (+ _output_get_2 (Math|Vector|MakeVector _returnvalue 0.0 0.0))))))
    (:then_1
      (Variables|Default|SetBP_FirstPerson (.AsBP%20First%20Person%20Character (Utilities|Casting|CastToBP_FirstPersonCharacter (Game|Player|GetPlayerPawn 0)))))))

(event Collision|EventActorBeginOverlap
  (params (OtherActor :type Actor%20Object%20Reference)))

(fn ConstructionScript)