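; BP_BulletBase is a bullet actor that explodes on impact and triggers target dummy reactions.
; On a blocking hit of its collision sphere, it attaches an explosion particle to the Sphere component, then destroys itself after a short delay.
; The same hit also checks for a "Dummy" component tag and, through a DoOnce, calls HitBehaviour on the owning BP_TargetDummy.
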(event OnComponentHit(SphereCollision)
  (params (HitComponent :type Primitive%20Component%20Object%20Reference) (OtherActor :type Actor%20Object%20Reference) (OtherComp :type Primitive%20Component%20Object%20Reference) (NormalImpulse :type Vector :default "0, 0, 0") (Hit :type Hit%20Result%20Structure%20%28by%20ref%29))
  (bind (_bblockinghit _binitialoverlap _time _distance _location _impactpoint _normal _impactnormal _physmat _hitactor _hitcomponent) (Collision|BreakHitResult Hit))
  (Utilities|FlowControl|Sequence
    (:then_0
      (if _bblockinghit
        (Effects|SpawnEmitterAttached "/Game/StarterContent/Particles/P_Explosion.P_Explosion" (Variables|Default|GetSphere) "None")
        (Utilities|FlowControl|Delay 0.25)
        (Actor|DestroyActor)))
    (:then_1
      (if (Components|ComponentHasTag _hitcomponent "Dummy")
        (Utilities|FlowControl|DoOnce false
          (:Completed
            (Default|HitBehaviour (.AsBP%20Target%20Dummy (Utilities|Casting|CastToBP_TargetDummy (Components|GetOwner _hitcomponent))))))))))

(event EventBeginPlay)

(event Collision|EventActorBeginOverlap
  (params (OtherActor :type Actor%20Object%20Reference)))

(event EventTick
  (params (DeltaSeconds :type Float%20%28single-precision%29)))

(fn ConstructionScript)